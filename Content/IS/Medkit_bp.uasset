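; Medkit pickup actor that heals the player or goes into their inventory.
; When its Box is overlapped by a ThirdPersonCharacter, it checks that character's FullHealth.
; At full health it increments MedKitAmount, otherwise it restores a fixed amount of health, clamped to the maximum.
; Either branch destroys the pickup and prints an on-screen message.
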(event `self.Box.OnComponentBeginOverlap`
  (params (OverlappedComponent :type "PrimitiveComponent Object Reference") (OtherActor :type "Actor Object Reference") (OtherComp :type "PrimitiveComponent Object Reference") (OtherBodyIndex :type Integer) (bFromSweep :type Boolean) (SweepResult :type "HitResult Structure (by ref)"))
  (bind _asthird_person_character (cast `/Game/ThirdPersonBP/Blueprints/ThirdPersonCharacter` OtherActor))
  (if (>= (`/Game/ThirdPersonBP/Blueprints/ThirdPersonCharacter.FullHealth` _asthird_person_character) 100.0)
    (set `/Game/ThirdPersonBP/Blueprints/ThirdPersonCharacter.MedKit Amount` (+ (`/Game/ThirdPersonBP/Blueprints/ThirdPersonCharacter.MedKit Amount` _asthird_person_character) 1) _asthird_person_character)
    (`KismetSystemLibrary.PrintString` "Medkit added to inventory")
    (`self.K2_DestroyActor`)
    (else
      (set `/Game/ThirdPersonBP/Blueprints/ThirdPersonCharacter.FullHealth` (`KismetMathLibrary.FMin` (+ (`/Game/ThirdPersonBP/Blueprints/ThirdPersonCharacter.FullHealth` _asthird_person_character) 25.0) 100.0) _asthird_person_character)
      (`self.K2_DestroyActor`)
      (`KismetSystemLibrary.PrintString` "you have found a medkit"))))

(fn `UserConstructionScript`)