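; Medkit pickup actor that adds a medkit to the player Victim's inventory when touched.
; A box overlap casts the other actor to Victim, increments its MedKitAmount, prints a confirmation and destroys the pickup.
; Tick spins the Medkit component by adding a fixed yaw each frame, so the rotation speed depends on frame rate.
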(event `self.Box.OnComponentBeginOverlap`
  (params (OverlappedComponent :type "PrimitiveComponent Object Reference") (OtherActor :type "Actor Object Reference") (OtherComp :type "PrimitiveComponent Object Reference") (OtherBodyIndex :type Integer) (bFromSweep :type Boolean) (SweepResult :type "HitResult Structure (by ref)"))
  (bind _asvictim (cast `/Game/ThirdPersonBP/Blueprints/Victim` OtherActor))
  (set `/Game/ThirdPersonBP/Blueprints/Victim.MedKit Amount` (+ (`/Game/ThirdPersonBP/Blueprints/Victim.MedKit Amount` _asvictim) 1) _asvictim)
  (`KismetSystemLibrary.PrintString` "medkit added to inventory")
  (`self.K2_DestroyActor`))

(event `self.ReceiveTick`
  (params (DeltaSeconds :type "Float (single-precision)"))
  (bind _medkit (`self.medkit`))
  (bind (_returnvalue_roll _returnvalue_pitch _returnvalue_yaw) (`KismetMathLibrary.BreakRotator` (`SceneComponent.K2_GetComponentRotation` _medkit)))
  (`SceneComponent.K2_SetWorldRotation` _medkit (`KismetMathLibrary.MakeRotator` _returnvalue_roll _returnvalue_pitch (+ _returnvalue_yaw 0.5)) false false))

(fn `UserConstructionScript`)