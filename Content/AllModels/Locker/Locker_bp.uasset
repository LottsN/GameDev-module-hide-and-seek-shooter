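; Locker Blueprint with a door that the player opens with the OpenDoor input while standing inside its trigger box.
; Overlapping the box as the ThirdPersonCharacter enables the locker's input, and leaving disables it and reverses the timeline.
; The Forlocker timeline drives the LockerDoor's relative rotation by lerping between StartRotation and EndRotation, so the door swings shut when the character walks away.
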(event `self.Box.OnComponentBeginOverlap`
  (params (OverlappedComponent :type "PrimitiveComponent Object Reference") (OtherActor :type "Actor Object Reference") (OtherComp :type "PrimitiveComponent Object Reference") (OtherBodyIndex :type Integer) (bFromSweep :type Boolean) (SweepResult :type "HitResult Structure (by ref)"))
  (cast `/Game/ThirdPersonBP/Blueprints/ThirdPersonCharacter` OtherActor)
  (`self.EnableInput` (`GameplayStatics.GetPlayerController` 0)))

(event `InputAction|OpenDoor`
  (params (Key :type "Key Structure"))
  (:`Pressed`
    (bind (_direction _lockerrotation) (`Timeline|forlocker` :!label _label)
      (:`Update`
        (`SceneComponent.K2_SetRelativeRotation` (`self.Locker_Door`) (`KismetMathLibrary.RLerp` (`self.start_rotation`) (`self.end_rotation`) _lockerrotation) false false)))))

(event `self.Box.OnComponentEndOverlap`
  (params (OverlappedComponent :type "PrimitiveComponent Object Reference") (OtherActor :type "Actor Object Reference") (OtherComp :type "PrimitiveComponent Object Reference") (OtherBodyIndex :type Integer))
  (cast `/Game/ThirdPersonBP/Blueprints/ThirdPersonCharacter` OtherActor)
  (`self.DisableInput` (`GameplayStatics.GetPlayerController` 0))
  (goto _label :!via `Reverse`))

(fn `UserConstructionScript`)