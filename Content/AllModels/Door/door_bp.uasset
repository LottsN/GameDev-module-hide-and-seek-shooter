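; Interactive door Blueprint that lets the player, when playing as a Victim, swing a school door open and closed.
; Overlapping the Box enables input for player controller 0, and leaving it disables input.
; Each OpenDoor press passes a Victim cast, then a FlipFlop alternates playing and reversing a timeline that lerps the door mesh's relative rotation between StartRotation and EndRotation.
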(event `InputAction|OpenDoor`
  (params (Key :type "Key Structure"))
  (:`Pressed`
    (cast `/Game/ThirdPersonBP/Blueprints/Victim` (`GameplayStatics.GetPlayerCharacter` 0))
    (`/Engine/EditorBlueprintResources/StandardMacros.FlipFlop`
      (:`A`
        (bind (_direction _doorrotation) (`Timeline|Timeline_1` :!label _label)
          (:`Update`
            (`SceneComponent.K2_SetRelativeRotation` (`self.school_door_movable_door`) (`KismetMathLibrary.RLerp` (`self.startRotation`) (`self.endRotation`) _doorrotation) false false))))
      (:`B`
        (goto _label :!via `Reverse`)))))

(event `self.Box.OnComponentBeginOverlap`
  (params (OverlappedComponent :type "PrimitiveComponent Object Reference") (OtherActor :type "Actor Object Reference") (OtherComp :type "PrimitiveComponent Object Reference") (OtherBodyIndex :type Integer) (bFromSweep :type Boolean) (SweepResult :type "HitResult Structure (by ref)"))
  (`self.EnableInput` (`GameplayStatics.GetPlayerController` 0)))

(event `self.Box.OnComponentEndOverlap`
  (params (OverlappedComponent :type "PrimitiveComponent Object Reference") (OtherActor :type "Actor Object Reference") (OtherComp :type "PrimitiveComponent Object Reference") (OtherBodyIndex :type Integer))
  (`self.DisableInput` (`GameplayStatics.GetPlayerController` 0)))

(fn `UserConstructionScript`)