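; Kevlar armor pickup that adds to the Victim character's inventory.
; When a Victim overlaps its Box, it increments that character's KevlarAmount by one, prints a debug message and destroys itself.
; Every Tick it spins the armor and helmet meshes by adding a fixed yaw step, so the rotation speed depends on frame rate.
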(event `self.Box.OnComponentBeginOverlap`
  (params (OverlappedComponent :type "PrimitiveComponent Object Reference") (OtherActor :type "Actor Object Reference") (OtherComp :type "PrimitiveComponent Object Reference") (OtherBodyIndex :type Integer) (bFromSweep :type Boolean) (SweepResult :type "HitResult Structure (by ref)"))
  (bind _asvictim (cast `/Game/ThirdPersonBP/Blueprints/Victim` OtherActor))
  (set `/Game/ThirdPersonBP/Blueprints/Victim.Kevlar Amount` (+ (`/Game/ThirdPersonBP/Blueprints/Victim.Kevlar Amount` _asvictim) 1) _asvictim)
  (`KismetSystemLibrary.PrintString` "kevlar added to inventory")
  (`self.K2_DestroyActor`))

(event `self.ReceiveTick`
  (params (DeltaSeconds :type "Float (single-precision)"))
  (bind _armor_armor (`self.armor_armor`))
  (bind _armor_helmet (`self.armor_helmet`))
  (bind (_returnvalue_roll _returnvalue_pitch _returnvalue_yaw) (`KismetMathLibrary.BreakRotator` (`SceneComponent.K2_GetComponentRotation` _armor_helmet)))
  (bind (_returnvalue_roll_2 _returnvalue_pitch_2 _returnvalue_yaw_2) (`KismetMathLibrary.BreakRotator` (`SceneComponent.K2_GetComponentRotation` _armor_armor)))
  (`SceneComponent.K2_SetWorldRotation` _armor_armor (`KismetMathLibrary.MakeRotator` _returnvalue_roll_2 _returnvalue_pitch_2 (+ _returnvalue_yaw_2 0.5)) false false)
  (`SceneComponent.K2_SetWorldRotation` _armor_helmet (`KismetMathLibrary.MakeRotator` _returnvalue_roll _returnvalue_pitch (+ _returnvalue_yaw 0.5)) false false))

(fn `UserConstructionScript`)